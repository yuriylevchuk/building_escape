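; BP_OpenableDoor is a door actor that swings open and closed in response to OnOpen and OnClose events from its OpenDoor component.
; It stores its starting rotation on BeginPlay, and the DoorSwing timeline adds an animated yaw offset to it.
; An event track on the timeline plays a sound at the door's location, and closing runs the same timeline in reverse.
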(event `self.ReceiveBeginPlay`
  (set `self.InitialRotation` (`self.K2_GetActorRotation`)))

(event `self.OpenDoor.OnOpen`
  (bind (_direction _openangle) (`Timeline|Door Swing` :!label _label)
    (:`Update`
      (`self.K2_SetActorRotation` (`KismetMathLibrary.ComposeRotators` (`KismetMathLibrary.MakeRotator` 0.0 0.0 _openangle) (`self.InitialRotation`))))
    (:`Sound`
      (`GameplayStatics.PlaySoundAtLocation` "/Game/Audio/Sound_08433.Sound_08433" (`self.K2_GetActorLocation`) (struct) 1.0 1.0 0.0 null null null))))

(event `self.OpenDoor.OnClose`
  (goto _label :!via `Reverse`))

(fn `UserConstructionScript`)